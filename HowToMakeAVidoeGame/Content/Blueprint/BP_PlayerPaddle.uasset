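; BP_PlayerPaddle is the player-controlled paddle that also spawns the game's ball.
; The HorizontalMovement input axis drives a physics impulse on the Paddle component along the X axis, scaled by Speed.
; The NewBall event, called on BeginPlay, spawns a BP_Ball at the Arrow component's transform and stores it in Ball.
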(event Custom|NewBall
  ;[1 1 1] SpawnBall
  (bind _returnvalue (Game|SpawnActorfromClass "/Game/Blueprint/BP_Ball.BP_Ball_C" (Transformation|GetWorldTransform (Variables|Default|GetArrow)) "Undefined" 0 0))
  (Variables|Default|SetBall _returnvalue))

(event EventBeginPlay
  (CallFunction|NewBall))

(event Input|AxisEvents|InputAxisHorizontalMovement
  (params (AxisValue :type Float%20%28single-precision%29))
  ;[1 1 1] PaddleMovement
  (Physics|AddImpulse (Variables|Default|GetPaddle) (Math|Vector|MakeVector (* AxisValue (Variables|Default|GetSpeed)) 0.0 0.0) "None" false))

(fn ConstructionScript)